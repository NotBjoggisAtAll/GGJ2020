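; BP_BuilderBob is the AI-driven Bob character that gathers collectibles and wins the level at the finish flag.
; Capsule overlaps handle pickups with normal or random "meme" sounds, and destroy Bob on anything other than collectibles, interactables or the flag.
; The flag triggers effects, the victory screen and walk end, then saves collectibles under the level-name number if new or improved.
; Hitting a horizontal red beam stops physics and keeps only yaw.
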(event OnComponentHit(CapsuleComponent)
  (params (HitComponent :type Primitive%20Component%20Object%20Reference) (OtherActor :type Actor%20Object%20Reference) (OtherComp :type Primitive%20Component%20Object%20Reference) (NormalImpulse :type Vector :default "0, 0, 0") (Hit :type Hit%20Result%20Structure%20%28by%20ref%29))
  (bind _asbp_red_beam (Utilities|Casting|CastToBP_RedBeam OtherActor))
  (if (Variables|/Game/Blueprints/BP_RedBeam.BP_RedBeam_C|GetIsHorizontal _asbp_red_beam)
    (Physics|SetSimulatePhysics (Variables|Default|GetCapsuleComponent) false)
    (Transformation|SetActorRotation (Math|Rotator|MakeRotator 0.0 0.0 (.yaw (Transformation|GetActorRotation))))))

(event OnComponentBeginOverlap(CapsuleComponent)
  (params (OverlappedComponent :type Primitive%20Component%20Object%20Reference) (OtherActor :type Actor%20Object%20Reference) (OtherComp :type Primitive%20Component%20Object%20Reference) (OtherBodyIndex :type Integer) (bFromSweep :type Boolean) (SweepResult :type Hit%20Result%20Structure%20%28by%20ref%29))
  (bind _returnvalue (Transformation|GetActorLocation))
  (bind _returnvalue_2 (Transformation|GetActorLocation))
  (bind (_asbp_finish_flag _bsuccess) (Utilities|Casting|CastToBP_FinishFlag OtherActor))
  (bind (_ascollectible _bsuccess_2) (Utilities|Casting|CastToCollectible OtherActor))
  (bind _collection (Variables|Default|GetCollection))
  (bind _soundeffectsonpickup (Variables|Default|GetSoundeffectsonpickup))
  (if _bsuccess_2
    (Class|BuilderBob|OnCollected _ascollectible)
    (bind _ascustom_game_instance (Utilities|Casting|CastToCustomGameInstance (Game|GetGameInstance)))
    (if (Variables|/Script/GGJ2020.CustomGameInstance|GetbMemeify _ascustom_game_instance)
      (Audio|PlaySoundatLocation (Utilities|Array|Get(acopy) _soundeffectsonpickup (Math|Random|RandomIntegerinRange 0 (- (Utilities|Array|Length _soundeffectsonpickup) 1))) _returnvalue "0, 0, 0" 1.0 1.0 0.0 0 0 0)
      (else
        (Audio|PlaySoundatLocation "/Game/Sounds/Collect.Collect" _returnvalue "0, 0, 0" 1.0 1.0 0.0 0 0 0)))
    (elif (not (.bSuccess (Utilities|Casting|CastToBaseInteractable OtherActor)))
      (if _bsuccess
        (Niagara|SpawnSystematLocation "/Game/Particles/Confetti_System.Confetti_System" _returnvalue_2)
        (Audio|PlaySoundatLocation "/Game/Sounds/Eating2_Cue.Eating2_Cue" _returnvalue_2 "0, 0, 0" 1.0 1.0 0.0 0 0 0)
        (Actor|DestroyActor _asbp_finish_flag)
        (bind _asbp_build_controller (Utilities|Casting|CastToBP_BuildController (Game|GetPlayerController 0)))
        (bind _returnvalue_3 (UserInterface|CreateWidget "/Game/UI/VictoryScreen.VictoryScreen_C" _asbp_build_controller))
        (UserInterface|Viewport|AddtoViewport _returnvalue_3 0)
        (Input|SetInputModeUIOnly _asbp_build_controller 0 "DoNotLock")
        (Variables|/Script/Engine.PlayerController|SetbShowMouseCursor _asbp_build_controller true)
        (Rendering|SetVisibility (Variables|/Script/GGJ2020.BaseInteractable|GetMesh (Variables|/Script/GGJ2020.BuildController|GetCurrentInteractable _asbp_build_controller)) false false)
        (bind _asbp_bob_controller (Utilities|Casting|CastToBP_BobController (AI|GetAIController self)))
        (Default|EndWalk _asbp_bob_controller)
        (Variables|Default|SetBobWon true)
        (Transformation|SetActorRotation "0,90.000000, 0")
        ;[1 1 1] Save
        (bind _returnvalue_4 (Game|GetCurrentLevelName true))
        (bind _result (Math|Integer|DecrementInt (Class|KismetSystemLibrary|MakeLiteralInteger (Math|Conversions|ToInteger(Byte) (.RightS (Utilities|String|Split _returnvalue_4 "_")))))
          (:%20%20
            (bind _ascustom_game_instance_2 (Utilities|Casting|CastToCustomGameInstance (Game|GetGameInstance)))
            (if (< _result (Utilities|Array|Length (Variables|/Script/GGJ2020.CustomSaveGame|GetLevels (Variables|/Script/GGJ2020.CustomGameInstance|GetSaveGame _ascustom_game_instance_2))))
              (if (> (Utilities|Array|Length _collection) (Utilities|Array|Length (.Collected (Utilities|Struct|BreakLevelData (Utilities|Array|Get(acopy) (Variables|/Script/GGJ2020.CustomSaveGame|GetLevels (Variables|/Script/GGJ2020.CustomGameInstance|GetSaveGame _ascustom_game_instance_2)) _result)))))
                (|SetBy-RefVar (.Collected (Utilities|Struct|BreakLevelData (Utilities|Array|Get(acopy) (Variables|/Script/GGJ2020.CustomSaveGame|GetLevels (Variables|/Script/GGJ2020.CustomGameInstance|GetSaveGame _ascustom_game_instance_2)) _result))) (Variables|Default|GetCollection))
                (Class|CustomGameInstance|Save _ascustom_game_instance_2 :!label _label))
              (else
                (Utilities|Array|Add (Variables|/Script/GGJ2020.CustomSaveGame|GetLevels (Variables|/Script/GGJ2020.CustomGameInstance|GetSaveGame _ascustom_game_instance_2)) (Utilities|Struct|MakeLevelData (Class|KismetSystemLibrary|MakeLiteralInteger (Math|Conversions|ToInteger(Byte) (.RightS (Utilities|String|Split _returnvalue_4 "_")))) _collection (Utilities|Array|Length (Variables|Default|GetWorldCollectibles))))
                (goto _label)))))
        (else
          (Actor|DestroyActor))))))

(fn ConstructionScript)