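; BP_BuildController is a player controller that handles the start-of-play screen and the pause menu.
; BeginPlay shows the BeforePlay widget; the StartPlay input removes it and tells the BP_BobController actor to begin walking.
; The Pause input opens PauseMenu, switches to UI-only input with a visible cursor, hides the current interactable's mesh and pauses the game.
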(event EventBeginPlay
  (bind _returnvalue (UserInterface|CreateWidget "/Game/UI/BeforePlay.BeforePlay_C" self))
  (bind _output_get (Variables|Default|SetBeforePlayScreen _returnvalue))
  (UserInterface|Viewport|AddtoViewport _output_get 0))

(event EventTick
  (params (DeltaSeconds :type Float%20%28single-precision%29)))

(event Input|ActionEvents|InputActionPause
  (params (Key :type Key%20Structure :default "None"))
  (bind _self self)
  (:Pressed
    (bind _returnvalue (UserInterface|CreateWidget "/Game/UI/PauseMenu.PauseMenu_C" _self))
    (UserInterface|Viewport|AddtoViewport _returnvalue 0)
    (Input|SetInputModeUIOnly _self 0 "LockAlways")
    (Variables|Default|SetbShowMouseCursor true)
    (Rendering|SetVisibility (Variables|/Script/GGJ2020.BaseInteractable|GetMesh (Variables|Default|GetCurrentInteractable)) false false)
    (Game|SetGamePaused true)))

(event Input|ActionEvents|InputActionStartPlay
  (params (Key :type Key%20Structure :default "None"))
  (bind _beforeplayscreen (Variables|Default|GetBeforePlayScreen))
  (:Pressed
    (Utilities|IsValid _beforeplayscreen
      (:Is%20Valid
        (Widget|RemovefromParent _beforeplayscreen)
        (bind _returnvalue (Actor|GetActorOfClass "/Game/Blueprints/AI/BP_BobController.BP_BobController_C"))
        (Default|BeginWalk _returnvalue)))))

(fn ConstructionScript)