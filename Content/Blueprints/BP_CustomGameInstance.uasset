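; BP_CustomGameInstance is a custom Game Instance that starts the game's background music through StartMusic.
; StartMusic stops any valid existing AudioComp, then uses the Memeify flag to pick either the quieter HardMemes cue or the JT70sPawn_T111 cue.
; The chosen cue becomes a new 2D sound that persists across level transitions, is stored in AudioComp and plays from the beginning.
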(fn StartMusic
  (Utilities|IsValid (Variables|Default|GetAudioComp)
    (:Is%20Valid
      (Audio|Components|Audio|Stop (Variables|Default|GetAudioComp)))
    (:Is%20Not%20Valid
      _))
  (if (Variables|Default|GetbMemeify)
    (bind _returnvalue (Audio|CreateSound2D "/Game/Sounds/HardMemes_Cue.HardMemes_Cue" 0.3 1.0 0.0 0 true))
    (bind _output_get (Variables|Default|SetAudioComp _returnvalue))
    (Audio|Components|Audio|Play _output_get 0.0)
    (else
      (bind _returnvalue_2 (Audio|CreateSound2D "/Game/Sounds/JT70sPawn_T111_Cue.JT70sPawn_T111_Cue" 1.0 1.0 0.0 0 true))
      (bind _output_get_2 (Variables|Default|SetAudioComp _returnvalue_2))
      (Audio|Components|Audio|Play _output_get_2 0.0))))