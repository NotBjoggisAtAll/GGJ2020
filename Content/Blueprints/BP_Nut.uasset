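; BP_Nut is a Blueprint that periodically switches a panning effect on and off in its mesh's material.
; On BeginPlay it creates a dynamic material instance for the first material slot and starts a looping timer at the TimeBetween interval.
; Each tick of the timer flips CanPan and sets the matching material scalar to a fixed on or off value.
; The CanPanToggle function and construction script are empty.
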(event Custom|CustomEvent_0
  (bind _output_get (Variables|Default|SetCanPan (not (Variables|Default|GetCanPan))))
  (if _output_get
    (Rendering|Material|SetScalarParameterValue (Variables|Default|GetMaterial) "CanPan" (Math|Float|MakeLiteralFloat 3.0) :!class /Script/Engine.MaterialInstanceDynamic)
    (else
      (Rendering|Material|SetScalarParameterValue (Variables|Default|GetMaterial) "CanPan" (Math|Float|MakeLiteralFloat 0.0) :!class /Script/Engine.MaterialInstanceDynamic))))

(event EventBeginPlay
  (bind _mesh (Variables|Character|GetMesh))
  (bind _returnvalue (Rendering|Material|CreateDynamicMaterialInstance (Rendering|Material|GetMaterial _mesh 0) "None" :!class /Script/Engine.KismetMaterialLibrary))
  (Variables|Default|SetMaterial _returnvalue)
  (Rendering|Material|SetMaterial _mesh 0 _returnvalue)
  (Utilities|Time|SetTimerbyEvent (delegate Custom|CustomEvent_0) (Variables|Default|GetTimeBetween) true))

(fn ConstructionScript)

(fn CanPanToggle)