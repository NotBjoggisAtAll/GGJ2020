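; Behavior tree task that walks the BP_BuilderBob pawn left or right along the world X axis.
; On execute it caches the controlled pawn as Bob.
; Each tick it adds movement input, picking the Right or Left scale from Bob's MoveRight flag and doubling it while SpeedBoost is set.
; The task never calls Finish Execute, so it does not end by itself.
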(event EventReceiveTickAI
  (params (OwnerController :type AI%20Controller%20Object%20Reference) (ControlledPawn :type Pawn%20Object%20Reference) (DeltaSeconds :type Float%20%28single-precision%29))
  (bind _bob (Variables|Default|GetBob))
  (bind _left (Variables|Default|GetLeft))
  (bind _right (Variables|Default|GetRight))
  (bind _bmoveright (Variables|/Script/GGJ2020.BuilderBob|GetbMoveRight _bob))
  (bind _returnvalue (select _bmoveright _right _left))
  (Pawn|Input|AddMovementInput ControlledPawn "1.000000,0.000000, 0" (select (Variables|/Script/GGJ2020.BuilderBob|GetbSpeedBoost _bob) (* _returnvalue 2.0) _returnvalue) false))

(event EventReceiveExecuteAI
  (params (OwnerController :type AI%20Controller%20Object%20Reference) (ControlledPawn :type Pawn%20Object%20Reference))
  (bind (_asbp_builder_bob _bsuccess) (Utilities|Casting|CastToBP_BuilderBob ControlledPawn))
  (if _bsuccess
    (Variables|Default|SetBob _asbp_builder_bob)))