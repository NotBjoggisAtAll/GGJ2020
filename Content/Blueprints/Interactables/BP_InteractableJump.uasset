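; BP_InteractableJump is a jump interactable that recolors its mesh to show placement validity.
; Its SetMaterial event switches on a material type to apply default, can-place or cannot-place variants of the warning-stripe and neon materials to specific mesh slots.
; The construction script is empty, and the Blueprint's graphs contain no jump logic.
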(event EventSetMaterial
  (params (MaterialType :type EMaterialType%20Enum :default "Default"))
  (bind _mesh (Variables|Character|GetMesh))
  (switch Utilities|FlowControl|Switch|SwitchonEMaterialType MaterialType
    (:Default
      (Rendering|Material|SetMaterial _mesh 0 "/Game/Materials/M_WarningStripes_Default.M_WarningStripes_Default")
      (Rendering|Material|SetMaterial _mesh 1 "/Game/Materials/M_Neon_Default.M_Neon_Default")
      (Rendering|Material|SetMaterial _mesh 3 "/Game/Materials/M_Neon_Default.M_Neon_Default"))
    (:CanPlace
      (Rendering|Material|SetMaterial _mesh 0 "/Game/Materials/M_WarningStripes_CanPlace.M_WarningStripes_CanPlace")
      (Rendering|Material|SetMaterial _mesh 1 "/Game/Materials/M_Neon_CanPlace.M_Neon_CanPlace")
      (Rendering|Material|SetMaterial _mesh 3 "/Game/Materials/M_Neon_CanPlace.M_Neon_CanPlace"))
    (:CanNotPlace
      (Rendering|Material|SetMaterial _mesh 0 "/Game/Materials/M_WarningStripes_CantPlace.M_WarningStripes_CantPlace")
      (Rendering|Material|SetMaterial _mesh 1 "/Game/Materials/M_Neon_CantPlace.M_Neon_CantPlace")
      (Rendering|Material|SetMaterial _mesh 3 "/Game/Materials/M_Neon_CantPlace.M_Neon_CantPlace"))))

(fn ConstructionScript)